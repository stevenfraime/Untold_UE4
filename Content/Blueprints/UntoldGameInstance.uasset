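; UntoldGameInstance is a Game Instance Blueprint that handles multiplayer session creation, invite joining and teardown.
; CreateSession makes an Advanced Session and opens TheConstruct as a listen server.
; Accepted invites join the session, sharing the switch to game-only input with the host path, and failures print messages.
; DestroySession opens MainMenuMap before destroying the session.
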(event Custom|CreateSession
  (|AdvancedSession 0 (Game|GetPlayerController 0) 100 0 false true false true false true false false true
    (:OnSuccess
      (Game|OpenLevel(byName) "TheConstruct" true "listen")
      (Input|SetInputModeGameOnly (Game|GetPlayerController 0)))
    (:OnFailure
      (Development|PrintString "FAILED TO CREATE SESSION!" true true "(R=0.390625,G=0.000000,B=0.000000,A=1.000000)"))))

(event Custom|DestroySession
  (Game|OpenLevel(byName) "MainMenuMap")
  (|DestroySession (Game|GetPlayerController 0)))

(event EventOnSessionInviteAccepted
  (params (LocalPlayerNum :type Integer) (PersonInvited :type BP%20Unique%20Net%20Id%20Structure) (SessionToJoin :type Blueprint%20Session%20Result%20Structure%20%28by%20ref%29))
  (|JoinSession (Game|GetPlayerController 0) SessionToJoin
    (:OnSuccess
      (Input|SetInputModeGameOnly (Game|GetPlayerController 0)))
    (:OnFailure
      (Development|PrintString "FAILED TO JOIN SESSION!" true true "(R=0.390625,G=0.000000,B=0.000000,A=1.000000)"))))